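; Griffon status effect for the Lord of Beasts stance, a timed attack-for-defense trade that replaces the Golden Emperor effect.
; On apply, it raises attack, lowers defense and cuts the Stance Swap cooldown by CdReduction, then removes itself after EffectDuration.
; On removal, it reverses the buffs and shifts the cooldown again by CdReduction minus EffectDuration.
; It destroys itself if the target is not a FighterCharacter.
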(event EventOnEffectRemoved
  (params (Target :type General%20Character%20Object%20Reference))
  (bind _fightercharacter (Variables|Default|GetFighterCharacter))
  (Class|FighterCharacter|ForceChangeCdby _fightercharacter "Stance Swap" (* (+ (Variables|Default|GetEffectDuration) (* (Variables|Default|GetCdReduction) -1.0)) -1.0))
  (Class|FighterCharacter|ApplyBuff _fightercharacter (Utilities|Struct|MakeCharacterStatsBuffs 0.0 0.0 0.0 0.0 0.0 0.0 0.0 0.0 0.0 -1e+02 25.0 0.0 0.0 0.0)))

(event EventOnEffectApplied
  (params (Target :type General%20Character%20Object%20Reference))
  (Class|GeneralCharacter|RemoveStatusEffect Target "/Game/Characters/Fighters/Assets/Griffon/Blueprints/StatusEffects/SEGriffonGoldenEmperor_BP.SEGriffonGoldenEmperor_BP_C")
  (bind _asfighter_character (Utilities|Casting|CastToFighterCharacter Target)
    (:then
      (bind _output_get (Variables|Default|SetFighterCharacter _asfighter_character))
      (Class|FighterCharacter|ForceChangeCdby _output_get "Stance Swap" (* (Variables|Default|GetCdReduction) -1.0))
      (Class|FighterCharacter|ApplyBuff _output_get (Utilities|Struct|MakeCharacterStatsBuffs 0.0 0.0 0.0 0.0 0.0 0.0 0.0 0.0 0.0 1e+02 -25.0 0.0 0.0 0.0))
      ;[1 1 1] This effect only lasts for a certain amount of time
      (Utilities|FlowControl|Delay (Variables|Default|GetEffectDuration))
      (Class|GeneralCharacter|RemoveStatusEffect (Variables|Default|GetFighterCharacter) "SEGriffonLordOfBeasts_BP_C"))
    (:CastFailed
      (Components|DestroyComponent))))