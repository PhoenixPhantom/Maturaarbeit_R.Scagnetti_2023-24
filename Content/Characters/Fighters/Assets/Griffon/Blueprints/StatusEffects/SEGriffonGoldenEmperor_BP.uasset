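; Timed status effect for the Griffon fighter's Golden Emperor state, which replaces the Lord of Beasts effect on its target.
; On a FighterCharacter, it offsets the Stance Swap cooldown by negative CdReduction as soon as it is applied.
; After EffectDuration, it applies a second offset of CdReduction minus EffectDuration, then removes itself.
; On any other target, the component destroys itself.
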(event EventOnEffectApplied
  (params (Target :type General%20Character%20Object%20Reference))
  (bind _cdreduction (Variables|Default|GetCdReduction))
  (bind _effectduration (Variables|Default|GetEffectDuration))
  (bind _returnvalue (* _cdreduction -1.0))
  (Class|GeneralCharacter|RemoveStatusEffect Target "/Game/Characters/Fighters/Assets/Griffon/Blueprints/StatusEffects/SEGriffonLordOfBeasts_BP.SEGriffonLordOfBeasts_BP_C")
  (bind _asfighter_character (Utilities|Casting|CastToFighterCharacter Target)
    (:then
      (Class|FighterCharacter|ForceChangeCdby _asfighter_character "Stance Swap" _returnvalue)
      ;[1 1 1] This effect only lasts for a certain amount of time
      (Utilities|FlowControl|Delay _effectduration)
      (Class|FighterCharacter|ForceChangeCdby _asfighter_character "Stance Swap" (* (+ _effectduration _returnvalue) -1.0))
      (Class|GeneralCharacter|RemoveStatusEffect _asfighter_character "SEGriffonGoldenEmperor_BP_C"))
    (:CastFailed
      (Components|DestroyComponent))))