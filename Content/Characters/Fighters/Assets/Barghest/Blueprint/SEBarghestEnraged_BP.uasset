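; Status effect component that puts a fighter, by its name the Barghest, into an enraged state.
; On apply it switches the fighter's attack tree to Enraged, adds attack and defense buffs, sets a rage shell overlay material and enters a custom animation state.
; Removal reverses each change, cancelling the buffs with negative values.
; The component destroys itself if the target is not a FighterCharacter.
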(event EventOnEffectRemoved
  (params (Target :type General%20Character%20Object%20Reference))
  (bind _effecttargetfighter (Variables|Default|GetEffectTargetFighter))
  (Rendering|Material|SetOverlayMaterial (Variables|/Script/Engine.Character|GetMesh Target) 0 :!class /Script/Engine.MeshComponent)
  (Class|CustomAnimInstance|ExitCustomState (Variables|/Script/MAProject.GeneralCharacter|GetCustomAnimInstance Target) "CustomState0")
  (Class|FighterCharacter|SetAttackTreeMode _effecttargetfighter)
  ;[1 1 1] Remove the defense boost
  (Class|FighterCharacter|ApplyBuff _effecttargetfighter (Utilities|Struct|MakeCharacterStatsBuffs 0.0 0.0 0.0 0.0 0.0 0.0 0.0 0.0 0.0 -1e+02 -2e+02 0.0 0.0 0.0)))

(event EventOnEffectApplied
  (params (Target :type General%20Character%20Object%20Reference))
  (bind _asfighter_character (Utilities|Casting|CastToFighterCharacter Target)
    (:then
      (bind _output_get (Variables|Default|SetEffectTargetFighter _asfighter_character))
      (Class|FighterCharacter|SetAttackTreeMode _output_get "Enraged")
      ;[1 1 1] Add defense boost
      (Class|FighterCharacter|ApplyBuff _output_get (Utilities|Struct|MakeCharacterStatsBuffs 0.0 0.0 0.0 0.0 0.0 0.0 0.0 0.0 0.0 1e+02 2e+02 0.0 0.0 0.0))
      (Rendering|Material|SetOverlayMaterial (Variables|/Script/Engine.Character|GetMesh Target) "/Game/Characters/Fighters/Assets/Barghest/Materials/MInst_BarghestRageShell.MInst_BarghestRageShell" :!class /Script/Engine.MeshComponent)
      (Class|CustomAnimInstance|EnterCustomState (Variables|/Script/MAProject.GeneralCharacter|GetCustomAnimInstance Target) "CustomState0"))
    (:CastFailed
      (Components|DestroyComponent))))